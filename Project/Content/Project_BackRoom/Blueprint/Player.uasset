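; Player Blueprint for the BackRoom project, providing jump, toggleable night vision and stepped camera zoom, and creating the PHUD widget on BeginPlay.
; The V key swaps post-process settings between normal and night vision.
; While night vision is on, Tick drains NVBattery through a short Delay and restores normal settings when it is empty.
; Zoom inputs step the camera FOV, clamped between MinFOV and DefaultFOV.
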(event `self.ReceiveBeginPlay`
  (bind _returnvalue (`|CreateWidget` "/Game/Project_BackRoom/Blueprint/PHUD.PHUD_C"))
  (set `self.CurrentZoom` (`self.DefaultFOV`))
  (`UserWidget.AddToViewport` _returnvalue 0))

(event `self.ReceiveTick`
  (params (DeltaSeconds :type "Float (single-precision)"))
  (if (`self.IsNV`)
    (if (> (`self.NVBattery`) 0)
      (`KismetSystemLibrary.Delay` 0.2)
      (set `self.NVBattery` (- (`self.NVBattery`) 1))
      (else
        (set `PostProcessComponent.Settings` (`self.PP_Normal`) (`self.PostProcess`))
        (set `self.IsNV` false)))))

(event `Key|SpaceBar`
  (params (Key :type "Key Structure"))
  (:`Pressed`
    (`self.Jump`)))

(event `Key|V`
  (params (Key :type "Key Structure"))
  (:`Pressed`
    (if (`self.IsNV`)
      (set `PostProcessComponent.Settings` (`self.PP_Normal`) (`self.PostProcess`))
      (set `self.IsNV` false)
      (else
        (set `PostProcessComponent.Settings` (`self.PP_NV`) (`self.PostProcess`))
        (set `self.IsNV` true)))))

(event `InputAction|ZoomIn`
  (params (Key :type "Key Structure"))
  (bind _camera (`self.Camera`))
  (bind _returnvalue (- (`CameraComponent.FieldOfView` (`self.Camera`)) 10.0))
  ;[1 1 1] ZoomIn
  (:`Pressed`
    (if (< _returnvalue (`self.MinFOV`))
      (`CameraComponent.SetFieldOfView` _camera (`self.MinFOV`))
      (else
        (bind _output_get (set `self.CurrentZoom` _returnvalue))
        (`CameraComponent.SetFieldOfView` _camera _output_get)))))

(event `InputAction|ZoomOut`
  (params (Key :type "Key Structure"))
  (bind _camera (`self.Camera`))
  (bind _returnvalue (+ (`CameraComponent.FieldOfView` (`self.Camera`)) 10.0))
  ;[1 1 1] ZooOut
  (:`Pressed`
    (if (> _returnvalue (`self.DefaultFOV`))
      (`CameraComponent.SetFieldOfView` _camera (`self.DefaultFOV`))
      (else
        (bind _output_get (set `self.CurrentZoom` _returnvalue))
        (`CameraComponent.SetFieldOfView` _camera _output_get)))))

(fn `UserConstructionScript`)