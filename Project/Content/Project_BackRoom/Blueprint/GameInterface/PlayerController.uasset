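; Player controller that drives the controlled pawn's movement, look and sprint.
; Move axes add movement input along the pawn root component's forward and right vectors, scaled by a shared Speed variable, while Turn and LookUp add yaw and pitch input.
; Holding Left Shift raises Speed and releasing it lowers it, so sprinting works by scaling input rather than changing the pawn's max movement speed.
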(event `InputAxis|MoveForward`
  (params (AxisValue :type "Float (single-precision)"))
  (bind _returnvalue (`self.K2_GetPawn`))
  (`Pawn.AddMovementInput` _returnvalue (`SceneComponent.GetForwardVector` (`Actor.RootComponent` _returnvalue)) (* AxisValue (`self.speed`)) false))

(event `InputAxis|Turn`
  (params (AxisValue :type "Float (single-precision)"))
  (`self.AddYawInput` AxisValue))

(event `InputAxis|LookUp`
  (params (AxisValue :type "Float (single-precision)"))
  (`self.AddPitchInput` AxisValue))

(event `InputAxis|MoveRight`
  (params (AxisValue :type "Float (single-precision)"))
  (bind _returnvalue (`self.K2_GetPawn`))
  (`Pawn.AddMovementInput` _returnvalue (`SceneComponent.GetRightVector` (`Actor.RootComponent` _returnvalue)) (* (`self.speed`) AxisValue) false))

(event `Key|LeftShift`
  (params (Key :type "Key Structure"))
  (:`Pressed`
    (set `self.speed` 1.0))
  (:`Released`
    (set `self.speed` 0.2)))

(fn `UserConstructionScript`)