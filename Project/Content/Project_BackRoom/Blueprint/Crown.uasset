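; Crown is a pawn or character AI that waits idle until the player comes within a set 2D range, then moves continuously.
; Each Tick, SetDistandDir updates the player distance, and a State switch goes from Idle to Follow with no way back.
; Follow applies movement input along DirPlayer, which is normalized from the scalar distance rather than the offset to the player, so it does not point at the player.
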(event `self.ReceiveTick`
  (params (DeltaSeconds :type "Float (single-precision)"))
  (`self.SetDistandDir`)
  (switch `/Game/Project_BackRoom/Blueprint/CrownEnum` (`self.State`)
    (:`NewEnumerator0`
      (if (<= (`self.Dist`) 500.0)
        (set `self.State` "NewEnumerator1")))
    (:`NewEnumerator1`
      (`self.AddMovementInput` (`self.Dir Player`)))))

(fn `SetDistandDir`
  (bind (_returnvalue_x _returnvalue_y) (`KismetMathLibrary.BreakVector` (`self.K2_GetActorLocation`)))
  (bind (_returnvalue_x_2 _returnvalue_y_2) (`KismetMathLibrary.BreakVector` (`self.K2_GetActorLocation` (`GameplayStatics.GetPlayerCharacter` 0))))
  (bind _returnvalue (`KismetMathLibrary.Distance2D` (`KismetMathLibrary.MakeVector2D` _returnvalue_x_2 _returnvalue_y_2) (`KismetMathLibrary.MakeVector2D` _returnvalue_x _returnvalue_y)))
  (set `self.Dist` _returnvalue)
  (set `self.Dir Player` (`KismetMathLibrary.Vector_Normal2D` (`KismetMathLibrary.Conv_DoubleToVector` _returnvalue))))

(fn `UserConstructionScript`)