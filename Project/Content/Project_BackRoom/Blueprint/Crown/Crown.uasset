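; Crown is a clown jumpscare threat that sends the player to the "Die" level when its capsule overlaps them.
; The mesh is hidden on BeginPlay, while nothing in the graph disables the capsule's overlap.
; Visible, with no caller in this Blueprint, reveals the mesh, plays a laugh at the capsule, snaps it to a fixed rotation and loops a fast-run animation.
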(event `self.ReceiveBeginPlay`
  (`SceneComponent.SetVisibility` (`self.Mesh`) false false))

(event `self.ReceiveTick`
  (params (DeltaSeconds :type "Float (single-precision)")))

(event `self.CapsuleComponent.OnComponentBeginOverlap`
  (params (OverlappedComponent :type "PrimitiveComponent Object Reference") (OtherActor :type "Actor Object Reference") (OtherComp :type "PrimitiveComponent Object Reference") (OtherBodyIndex :type Integer) (bFromSweep :type Boolean) (SweepResult :type "HitResult Structure (by ref)"))
  (cast `/Game/Project_BackRoom/Blueprint/Player/Player` OtherActor)
  (`GameplayStatics.OpenLevel` "Die"))

(fn `UserConstructionScript`)

(fn `visible`
  (`SceneComponent.SetVisibility` (`self.Mesh`) true false)
  (`GameplayStatics.PlaySoundAtLocation` "/Game/Project_BackRoom/Sound/Clown_laugh_Cue.Clown_laugh_Cue" (`SceneComponent.K2_GetComponentLocation` (`self.CapsuleComponent`)) (struct) 1.0 1.0 0.0 null null null)
  (`SceneComponent.K2_SetWorldRotation` (`self.CapsuleComponent`) (struct :`Yaw` -90.0) false false)
  (`SkeletalMeshComponent.PlayAnimation` (`self.Mesh`) "/Game/Project_BackRoom/Crown/Animation/Fast_Run.Fast_Run" true))