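; CrownAI is the AI controller for the Crown enemy, a clown that follows the player once it perceives them.
; It runs the FollowingPlayer behavior tree on BeginPlay and feeds it through AI perception updates filtered by the Player actor tag.
; A successful sense stores the player in the TargetLocation blackboard object key and plays a 2D clown laugh, while losing the stimulus clears the key.
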(event `self.ReceiveBeginPlay`
  (`self.RunBehaviorTree` "/Game/Project_BackRoom/AI/FollowingPlayer.FollowingPlayer"))

(event `self.AIPerception.OnTargetPerceptionUpdated`
  (params (Actor :type "Actor Object Reference") (Stimulus :type "AIStimulus Structure"))
  (bind _blackboard (`self.Blackboard`))
  (if (`self.ActorHasTag` Actor "Player")
    (if (`.bSuccessfullySensed` (break `AIStimulus` Stimulus))
      (`BlackboardComponent.SetValueAsObject` _blackboard "TargetLocation" Actor)
      (`GameplayStatics.PlaySound2D` "/Game/Project_BackRoom/Sound/Clown_laugh_Cue.Clown_laugh_Cue" 1.0 1.0 0.0 null null)
      (else
        (`BlackboardComponent.SetValueAsObject` _blackboard "TargetLocation" null)))))

(fn `UserConstructionScript`)