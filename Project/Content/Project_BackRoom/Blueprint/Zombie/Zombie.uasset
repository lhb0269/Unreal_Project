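; Zombie actor that stays hidden from BeginPlay until revealed, and sends the player to the "Die" level on contact.
; The Visible function shows the mesh, sets the capsule's world rotation, loops the walking animation and plays a 2D zombie sound.
; Capsule overlap with the Player opens that level, with no check on whether the zombie has been revealed.
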(event `self.ReceiveBeginPlay`
  (`SceneComponent.SetVisibility` (`self.Mesh`) false false))

(event `self.CapsuleComponent.OnComponentBeginOverlap`
  (params (OverlappedComponent :type "PrimitiveComponent Object Reference") (OtherActor :type "Actor Object Reference") (OtherComp :type "PrimitiveComponent Object Reference") (OtherBodyIndex :type Integer) (bFromSweep :type Boolean) (SweepResult :type "HitResult Structure (by ref)"))
  (cast `/Game/Project_BackRoom/Blueprint/Player/Player` OtherActor)
  (`GameplayStatics.OpenLevel` "Die"))

(fn `UserConstructionScript`)

(fn `visible`
  (`SceneComponent.SetVisibility` (`self.Mesh`) true false)
  (`SceneComponent.K2_SetWorldRotation` (`self.CapsuleComponent`) (struct :`Yaw` 180.0) false false)
  (`SkeletalMeshComponent.PlayAnimation` (`self.Mesh`) "/Game/Project_BackRoom/Zombie/z_Walking.z_Walking" true)
  (`GameplayStatics.PlaySound2D` "/Game/Project_BackRoom/Sound/zombie_Cue.zombie_Cue" 1.0 1.0 0.0 null null))